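; BP_CelLight is a test light actor that feeds its position to an actor inside its sphere, apparently for cel shading.
; Every Tick it sends its location via LightBlendMessage to the first actor overlapping the Sphere; any others are ignored.
; The construction script calls SetLightMask, which is empty.
; Disconnected nodes remain from other approaches, including a one-light system writing radius and location to the PointLightPosition parameter collection.
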(event `self.ReceiveTick`
  (params (DeltaSeconds :type "Float (single-precision)"))
  (bind _output (`|GetArrayItem` (`PrimitiveComponent.GetOverlappingActors` (`self.Sphere`) null)))
  (`/Engine/EditorBlueprintResources/StandardMacros.IsValid` _output
    (:`Is Valid`
      (message `/Game/Anime/Blueprints/Test/BPI_LightBlend.LightBlend` _output (`self.K2_GetActorLocation`)))))

(event `self.Sphere.OnComponentBeginOverlap`
  (params (OverlappedComponent :type "PrimitiveComponent Object Reference") (OtherActor :type "Actor Object Reference") (OtherComp :type "PrimitiveComponent Object Reference") (OtherBodyIndex :type Integer) (bFromSweep :type Boolean) (SweepResult :type "HitResult Structure (by ref)")))

(event `self.ReceiveBeginPlay`)

(event `self.Sphere.OnComponentEndOverlap`
  (params (OverlappedComponent :type "PrimitiveComponent Object Reference") (OtherActor :type "Actor Object Reference") (OtherComp :type "PrimitiveComponent Object Reference") (OtherBodyIndex :type Integer)))

(fn `Set Light Mask`)

(fn `UserConstructionScript`
  (`self.Set Light Mask`))